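; Base character Blueprint that manages acquiring and switching weapons, granting a default BP_WeaponBase shortly after BeginPlay.
; Acquired weapons spawn in the inventory state, attach to the mesh socket named in their class defaults, then become the pending active weapon.
; A switch montage plays, and the hand-down notify event performs the swap between inventory and in-hand states.
; GetActiveWeaponAnims exposes the active weapon's idle and walk animations.
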(event Custom|AcquireNewWeapon
  (params (Weapon%20Class :type BP%20Weapon%20Base%20Class%20Reference))
  (bind _equipsocketname (Utilities|GetClassDefaults Weapon%20Class))
  (bind _self self)
  (bind _returnvalue (Game|SpawnActorfromClass Weapon%20Class (Transformation|GetSocketTransform (Variables|Character|GetMesh) _equipsocketname "RTS_World") "Undefined" "MultiplyWithRoot" _self _self))
  (Default|WeaponinInventory _returnvalue)
  (Transformation|AttachComponentToComponent _returnvalue (Variables|Character|GetMesh) _equipsocketname "SnapToTarget" "SnapToTarget" "SnapToTarget" true)
  (CallFunction|SwitchActiveWeaponto _returnvalue))

(event Custom|SwitchActiveWeaponTo
  (params (NewActiveWeapon :type BP%20Weapon%20Base%20Object%20Reference))
  (Variables|Default|SetPendingNextActiveWeapon NewActiveWeapon)
  (Animation|Montage|PlayMontage (Variables|Character|GetMesh) "/Game/PlayerAssets/Animations/ASM_WeaponSwitch.ASM_WeaponSwitch"))

(event Custom|WeaponSwitchHandDownNotify
  (Utilities|FlowControl|Sequence
    (:then_0
      (Utilities|IsValid (Variables|Default|GetCurrentActiveWeapon)
        (:Is%20Valid
          (Default|WeaponinInventory (Variables|Default|GetCurrentActiveWeapon)))))
    (:then_1
      (bind _output_get (Variables|Default|SetCurrentActiveWeapon (Variables|Default|GetPendingNextActiveWeapon)))
      (Default|WeaponinHand _output_get))))

(event EventBeginPlay
  (Utilities|FlowControl|Delay 2.0)
  (CallFunction|AcquireNewWeapon "/Game/Blueprints/Weapons/BP_WeaponBase.BP_WeaponBase_C"))

(event Collision|EventActorBeginOverlap
  (params (OtherActor :type Actor%20Object%20Reference)))

(event EventTick
  (params (DeltaSeconds :type Float%20%28single-precision%29)))

(fn ConstructionScript)

(fn GetActiveWeaponAnims
  (bind _currentactiveweapon (Variables|Default|GetCurrentActiveWeapon))
  (return (Variables|/Game/Blueprints/Weapons/BP_WeaponBase.BP_WeaponBase_C|GetIdleAnim _currentactiveweapon) (Variables|/Game/Blueprints/Weapons/BP_WeaponBase.BP_WeaponBase_C|GetWalkAnim _currentactiveweapon)))